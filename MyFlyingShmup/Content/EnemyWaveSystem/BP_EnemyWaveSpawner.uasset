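; Enemy wave spawner actor that runs the waves in WavesData in order, then shows the mission-complete end screen.
; After each wave's initial delay, it spawns that wave's enemy list at timed intervals, randomly between two limit points or at the boss point for boss waves.
; Destroyed events decrement a remaining count seeded from the spawn-step count, which is polled until zero to start the next wave.
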(event Custom|BeginSetofWaves
  (Variables|Default|SetCurrentSpawn 0)
  (CallFunction|NextWave))

(event Custom|NextWave
  (if (> (Variables|Default|GetCurrentWaveIndex) (Variables|Default|GetLastWaveIndex))
    (bind _returnvalue (UserInterface|CreateWidget "/Game/UI/WBP_EndScreen.WBP_EndScreen_C" (Game|GetPlayerController 0) true))
    (UserInterface|Viewport|AddtoViewport _returnvalue 0)
    (else
      (Utilities|FlowControl|Delay (Utilities|Struct|BreakS_Wave (Utilities|Array|Get(acopy) (Variables|/Game/EnemyWaveSystem/PDA_SetofWave.PDA_SetofWave_C|GetWaves (Variables|Default|GetWavesData)) (Variables|Default|GetCurrentWaveIndex))))
      (CallFunction|BeginSpawn))))

(event Custom|NextSpawn
  (if (== (Variables|Default|GetCurrentSpawn) (Variables|Default|GetNumberToSpawn))
    (if (== (Variables|Default|GetEnemiesRemaining) 0) :!label _label
      (Math|Integer|IncrementInt (Variables|Default|GetCurrentWaveIndex)
        (:%20%20
          (CallFunction|NextWave)))
      (else
        (Utilities|FlowControl|Delay 0.2)
        (goto _label)))
    (else
      (for _array_element (.enemies (Variables|Default|GetEnemiesToSpawn))
        (bind _returnvalue (Game|SpawnActorfromClass _array_element (Math|Transform|MakeTransform (select (Variables|Default|GetIsBossWave) (Transformation|GetWorldLocation (Variables|Default|GetBossSpawnPoint)) (Math|Vector|Lerp(Vector) (Transformation|GetWorldLocation (Variables|Default|GetLeftSpawn_Limit)) (Transformation|GetWorldLocation (Variables|Default|GetRightSpawn_Limit)) (Math|Random|RandomFloat))) (Transformation|GetActorRotation) "1.000000,1.000000,1.000000") "AlwaysSpawn" "MultiplyWithRoot" 0 0))
        (Game|BindEventtoOnDestroyed _returnvalue (delegate Custom|EnemyDestroyed)))
      (Math|Integer|IncrementInt (Variables|Default|GetCurrentSpawn)
        (:%20%20
          (Utilities|FlowControl|Delay (Variables|Default|GetTimeBetweenSpawns))
          (CallFunction|NextSpawn))))))

(event Custom|BeginSpawn
  (bind _wavesdata (Variables|Default|GetWavesData))
  (bind _currentwaveindex (Variables|Default|GetCurrentWaveIndex))
  (bind _waves (Variables|/Game/EnemyWaveSystem/PDA_SetofWave.PDA_SetofWave_C|GetWaves _wavesdata))
  (bind _output (Utilities|Array|Get(acopy) _waves _currentwaveindex))
  (bind (_timebetweensawns _numberofspawns _enemies _isbosswave) (Utilities|Struct|BreakS_Wave _output))
  (Variables|Default|SetCurrentSpawn 0)
  (Variables|Default|SetTimeBetweenSpawns _timebetweensawns)
  (bind _output_get (Variables|Default|SetNumberToSpawn _numberofspawns))
  (Variables|Default|SetEnemiesRemaining _output_get)
  (Variables|Default|SetEnemiesToSpawn _enemies)
  (Variables|Default|SetIsBossWave _isbosswave)
  (CallFunction|NextSpawn))

(event Custom|EnemyDestroyed
  (params (DestroyedActor :type Actor%20Object%20Reference))
  (Math|Integer|DecrementInt (Variables|Default|GetEnemiesRemaining)))

(event EventBeginPlay
  (Variables|Default|SetLastWaveIndex (Utilities|Array|LastIndex (Variables|/Game/EnemyWaveSystem/PDA_SetofWave.PDA_SetofWave_C|GetWaves (Variables|Default|GetWavesData))))
  (CallFunction|BeginSetofWaves))

(fn ConstructionScript)