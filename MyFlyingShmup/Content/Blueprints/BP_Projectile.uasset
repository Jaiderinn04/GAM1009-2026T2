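; BP_Projectile is a projectile that damages whatever actor it overlaps, then destroys itself.
; On overlap it applies its Damage value, crediting the Instigator's controller as event instigator and the Instigator as damage causer.
; The Instigator validity check runs after the damage and leads nowhere, and the player-state score message call is disconnected, so it never runs.
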(event Collision|EventActorBeginOverlap
  (params (OtherActor :type Actor%20Object%20Reference))
  (Game|Damage|ApplyDamage OtherActor (Variables|Default|GetDamage) (Pawn|GetController (Variables|Actor|GetInstigator)) (Variables|Actor|GetInstigator))
  (Utilities|FlowControl|Sequence
    (:then_0
      (bind _instigator (Variables|Actor|GetInstigator)
        (:then)
        (:else)))
    (:then_1
      (Actor|DestroyActor))))

(fn ConstructionScript)