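; Pickup actor that homes in on a collector and hands over its PickUpStats.
; CollectPickUp, sent by the pawn, turns on projectile movement homing toward that target's root component at raised max speed.
; While homing, sphere overlaps send a GetPickUpStats message to the other actor.
; The pickup's GetPickUpStats function returns its stats and triggers DestroySelf, which disables collision, hides it and destroys it after a short delay.
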(event OnComponentBeginOverlap(Sphere)
  (params (OverlappedComponent :type Primitive%20Component%20Object%20Reference) (OtherActor :type Actor%20Object%20Reference) (OtherComp :type Primitive%20Component%20Object%20Reference) (OtherBodyIndex :type Integer) (bFromSweep :type Boolean) (SweepResult :type Hit%20Result%20Structure%20%28by%20ref%29))
  (if (Variables|/Script/Engine.ProjectileMovementComponent|GetbIsHomingProjectile (Variables|Default|GetProjectileMovement))
    (Class|BPIMyFlyingShmup|GetPickUpStats(Message) OtherActor)))

(event Custom|DestroySelf
  (Collision|SetCollisionEnabled (Variables|Default|GetSphere) "NoCollision")
  (Rendering|SetActorHiddenInGame true)
  (Utilities|FlowControl|Delay 1.0)
  (Actor|DestroyActor))

(event Collision|EventActorBeginOverlap
  (params (OtherActor :type Actor%20Object%20Reference)))

(event EventCollectPickUp
  (params (HomingTarget :type Actor%20Object%20Reference))
  (bind _projectilemovement (Variables|Default|GetProjectileMovement))
  ;[0.15 0.15 0.15 0.5] Receive message from Pawn
  (Variables|/Script/Engine.ProjectileMovementComponent|SetHomingTargetComponent _projectilemovement (Variables|/Script/Engine.Actor|GetRootComponent HomingTarget))
  (Variables|/Script/Engine.ProjectileMovementComponent|SetbIsHomingProjectile _projectilemovement true)
  (Variables|/Script/Engine.ProjectileMovementComponent|SetMaxSpeed _projectilemovement 4e+03))

(fn ConstructionScript)

(fn GetPickUpStats
  (CallFunction|DestroySelf)
  (return (Variables|Default|GetPickUpStats)))