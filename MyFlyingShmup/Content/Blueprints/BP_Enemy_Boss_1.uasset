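; BP_Enemy_Boss_1 is a boss enemy that moves on an interpolated path while firing bullets on a repeating timer.
; On BeginPlay it runs the parent logic, then activates its InterpToMovementSideToSide component after a short delay.
; A looping timer, started without waiting for that delay, calls ShootBullet, which spawns BP_Projectile_EnemyBullet at the Arrow component's world location and rotation.
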(event Custom|ShootBullet
  (bind _arrow (Variables|Default|GetArrow))
  (bind _returnvalue (Transformation|GetWorldTransform _arrow))
  (Game|SpawnActorfromClass "/Game/Blueprints/BP_Projectile_EnemyBullet.BP_Projectile_EnemyBullet_C" (Math|Transform|MakeTransform (.location _returnvalue) (.rotation _returnvalue) "1.000000,1.000000,1.000000") "Undefined" "MultiplyWithRoot" 0 0))

(event EventBeginPlay
  (|CallParentFunction)
  (Utilities|FlowControl|Sequence
    (:then_0
      (Utilities|FlowControl|Delay 2.0)
      (Components|Activation|Activate (Variables|Default|GetInterpToMovement_SideToSide) false))
    (:then_1
      (Utilities|Time|SetTimerbyEvent (delegate Custom|ShootBullet) 0.9 true))))

(fn ConstructionScript
  (|CallParentFunction))