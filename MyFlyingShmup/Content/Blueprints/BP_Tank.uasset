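; BP_Tank is a player-controlled tank that drives, turns, rotates its gun and fires shells.
; W/S, A/D and Q/E open and close gates that Tick enters each frame, applying delta-time-scaled hull movement, hull turning or GunBody rotation.
; Driving moves without sweep and spins all four wheels, while turning spins only two.
; Space spawns BP_Tank_Shell at ShellSpawnPoint, and MouseX adds controller yaw.
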(event EventBeginPlay)

(event Collision|EventActorBeginOverlap
  (params (OtherActor :type Actor%20Object%20Reference)))

(event EventTick
  (params (DeltaSeconds :type Float%20%28single-precision%29))
  (Utilities|FlowControl|Sequence
    (:then_0
      (Utilities|FlowControl|Gate true
        (:Exit
          (Transformation|AddActorLocalOffset (* "100.000000,0.000000,0.000000" (Utilities|Time|GetWorldDeltaSeconds)) false false)
          (Transformation|AddLocalRotation (Variables|Default|GetWheel1) (* "0.000000,60.000000,0.000000" (Utilities|Time|GetWorldDeltaSeconds)) false false))))
    (:then_1
      (Utilities|FlowControl|Gate true
        (:Exit
          (Transformation|AddActorLocalOffset (* "-100.000000,0.000000,0.000000" (Utilities|Time|GetWorldDeltaSeconds)) false false)
          (Transformation|AddLocalRotation (Variables|Default|GetWheel1) (* "0.000000,-60.000000,0.000000" (Utilities|Time|GetWorldDeltaSeconds)) false false))))
    (:then_2
      (Utilities|FlowControl|Gate true
        (:Exit
          (Transformation|AddActorLocalRotation (* "0.000000,-60.000000,0.000000" (Utilities|Time|GetWorldDeltaSeconds)) false false)
          (Transformation|AddLocalRotation (Variables|Default|GetWheel) "0, 0, 0" false false)
          (Transformation|AddLocalRotation (Variables|Default|GetWheel1) (* "0.000000,-60.000000,0.000000" (Utilities|Time|GetWorldDeltaSeconds)) false false))))
    (:then_3
      (Utilities|FlowControl|Gate true
        (:Exit
          (Transformation|AddActorLocalRotation (* "0.000000,60.000000,0.000000" (Utilities|Time|GetWorldDeltaSeconds)) false false)
          (Transformation|AddLocalRotation (Variables|Default|GetWheel) "0, 0, 0" false false)
          (Transformation|AddLocalRotation (Variables|Default|GetWheel1) (* "0.000000,60.000000,0.000000" (Utilities|Time|GetWorldDeltaSeconds)) false false))))
    (:then_4
      (Utilities|FlowControl|Gate true
        (:Exit
          (Transformation|AddLocalRotation (Variables|Default|GetGunBody) (* "0.000000,-60.000000,0.000000" (Utilities|Time|GetWorldDeltaSeconds)) false false))))
    (:then_5
      (Utilities|FlowControl|Gate true
        (:Exit
          (Transformation|AddLocalRotation (Variables|Default|GetGunBody) (* "0.000000,60.000000,0.000000" (Utilities|Time|GetWorldDeltaSeconds)) false false))))))

(event Input|MouseEvents|MouseX
  (params (AxisValue :type Float%20%28single-precision%29))
  (Pawn|Input|AddControllerYawInput AxisValue))

(event Input|KeyboardEvents|SpaceBar
  (params (Key :type Key%20Structure :default "None"))
  (bind _shellspawnpoint (Variables|Default|GetShellSpawnPoint))
  (bind _returnvalue (Transformation|GetWorldTransform _shellspawnpoint))
  (:Pressed
    (Game|SpawnActorfromClass "/Game/Blueprints/BP_Tank_Shell.BP_Tank_Shell_C" (Math|Transform|MakeTransform (.location _returnvalue) (.rotation _returnvalue) "1.000000,1.000000,1.000000") "Undefined" "MultiplyWithRoot" 0 0)))

(event Input|KeyboardEvents|W
  (params (Key :type Key%20Structure :default "None"))
  (:Pressed
    (Utilities|FlowControl|Gate true) ; enters at Open
  )
  (:Released
    (Utilities|FlowControl|Gate true) ; enters at Close
  ))

(event Input|KeyboardEvents|S
  (params (Key :type Key%20Structure :default "None"))
  (:Pressed
    (Utilities|FlowControl|Gate true) ; enters at Open
  )
  (:Released
    (Utilities|FlowControl|Gate true) ; enters at Close
  ))

(event Input|KeyboardEvents|Q
  (params (Key :type Key%20Structure :default "None"))
  (:Pressed
    (Utilities|FlowControl|Gate true) ; enters at Open
  )
  (:Released
    (Utilities|FlowControl|Gate true) ; enters at Close
  ))

(event Input|KeyboardEvents|A
  (params (Key :type Key%20Structure :default "None"))
  (:Pressed
    (Utilities|FlowControl|Gate true) ; enters at Open
  )
  (:Released
    (Utilities|FlowControl|Gate true) ; enters at Close
  ))

(event Input|KeyboardEvents|D
  (params (Key :type Key%20Structure :default "None"))
  (:Pressed
    (Utilities|FlowControl|Gate true) ; enters at Open
  )
  (:Released
    (Utilities|FlowControl|Gate true) ; enters at Close
  ))

(event Input|KeyboardEvents|E
  (params (Key :type Key%20Structure :default "None"))
  (:Pressed
    (Utilities|FlowControl|Gate true) ; enters at Open
  )
  (:Released
    (Utilities|FlowControl|Gate true) ; enters at Close
  ))

(fn ConstructionScript)