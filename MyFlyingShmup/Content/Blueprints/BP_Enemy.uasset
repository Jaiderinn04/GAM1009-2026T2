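; BP_Enemy is an enemy actor that tracks health, takes damage and dies when health reaches zero.
; AnyDamage clamps health at zero, updates the WBP_EnemyHealthBar widget with the health ratio and spawns a BP_DamagePopUp at the actor's location.
; Surviving hits play a sound and temporarily apply an overlay material to the mesh.
; A lethal hit plays a kill sound, spawns BP_Explosion and destroys the actor.
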(event Custom|HitSecuence
  (Audio|PlaySound2D "/Game/Audio/MS_Hit.MS_Hit" 0.5 1.0 0.0 0 0)
  (Rendering|Material|SetOverlayMaterial (Variables|Default|GetStaticMesh) "/Game/Materials/M_Overlay.M_Overlay" :!class /Script/Engine.MeshComponent)
  (Utilities|FlowControl|Delay 2.0)
  ;[0.15 0.15 0.15 0.5] Health Check
  (Rendering|Material|SetOverlayMaterial (Variables|Default|GetStaticMesh) 0 :!class /Script/Engine.MeshComponent))

(event Custom|KillSequence
  (Audio|PlaySound2D "/Game/Audio/MS_Kill.MS_Kill" 0.5 1.0 0.0 0 0)
  (Game|SpawnActorfromClass "/Game/FX/BP_Explosion.BP_Explosion_C" (Math|Transform|MakeTransform (Transformation|GetActorLocation) "0, 0, 0" "1.000000,1.000000,1.000000") "AlwaysSpawn" "MultiplyWithRoot" 0 0)
  (Actor|DestroyActor))

(event EventBeginPlay)

(event Collision|EventActorBeginOverlap
  (params (OtherActor :type Actor%20Object%20Reference))
  (Utilities|FlowControl|Sequence))

(event Game|Damage|EventAnyDamage
  (params (Damage :type Float%20%28single-precision%29) (DamageType :type Damage%20Type%20Object%20Reference) (InstigatedBy :type Controller%20Object%20Reference) (DamageCauser :type Actor%20Object%20Reference))
  ;[0.15 0.15 0.15 0.5] BP_Projectile Applies Damage
  (Variables|Components|SetHealth (Math|Float|Max(Float) (- (Variables|Components|GetHealth) Damage) 0.0))
  (Utilities|FlowControl|Sequence
    (:then_0
      ;[0.15 0.15 0.15 0.5] Handles UI  Update
      (bind _aswbp_enemy_health_bar (Utilities|Casting|CastToWBP_EnemyHealthBar (UserInterface|GetUserWidgetObject (Variables|Default|GetWidget))))
      (Default|SetHealth _aswbp_enemy_health_bar (Math|Float|SafeDivide (Variables|Components|GetHealth) (Variables|Components|GetMaxHealth))))
    (:then_1
      (Game|SpawnActorfromClass "/Game/UI/BP_DamagePopUp.BP_DamagePopUp_C" (Math|Transform|MakeTransform (Transformation|GetActorLocation) "0, 0, 0" "1.000000,1.000000,1.000000") "Undefined" "MultiplyWithRoot" 0 Damage 0))
    (:then_2
      ;[0.15 0.15 0.15 0.5] Health Check
      (if (== (Variables|Components|GetHealth) 0.0)
        (CallFunction|KillSequence)
        (else
          (CallFunction|HitSecuence))))))

(fn ConstructionScript)